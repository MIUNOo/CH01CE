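; Interactable button that switches one set of spotlights off and, after a two-second delay, another set on.
; InteractWith plays a positional sound, then runs the sequence only if Triggered is already true, which nothing live clears.
; Each light change notifies the BP_LightSoundManager found at BeginPlay, and each switch-on plays a sound at that light.
; LookAt returns the button with an empty message.
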(event `self.ReceiveBeginPlay`
  (bind _returnvalue (`GameplayStatics.GetActorOfClass` "/Game/Audio/BP_LightSoundManager.BP_LightSoundManager_C"))
  (set `self.Light Sound Manager` _returnvalue))

(event `DelayTime`
  (params (sec :type "Float (double-precision)"))
  (`KismetSystemLibrary.Delay` sec)
  (`self.TurnLightsOn`))

(fn `InteractWith`
  (params (Interactor :type "Object Object Reference") (HitComponent :type "PrimitiveComponent Object Reference"))
  (returns (Interactable :type Boolean))
  (`GameplayStatics.PlaySoundAtLocation` null (`self.K2_GetActorLocation`) (struct) 1.0 1.0 0.0 null null null null)
  (if (not (not (`self.Triggered`)))
    (set `self.Triggered` true)
    (for _array_element (`self.LightsToTurnOff`)
      (`LightComponent.SetIntensity` (`SpotLight.SpotLightComponent` _array_element) 0.0)
      (`/Game/Audio/BP_LightSoundManager.Light Off` (`self.Light Sound Manager`)))
    (`self.DelayTime` 2.0))
  (return false))

(fn `LookAt`
  (params (Interactor :type "Object Object Reference") (Controller :type "PlayerController Object Reference") (HitComponent :type "PrimitiveComponent Object Reference"))
  (returns (LookAtActor :type "Actor Object Reference") (LookAtComponent :type "PrimitiveComponent Object Reference") (Message :type Text))
  (return self HitComponent ""))

(fn `TurnLightsOn`
  (for _array_element (`self.LightsToTurnOn`)
    (`LightComponent.SetIntensity` (`SpotLight.SpotLightComponent` _array_element) 160.0)
    (`GameplayStatics.PlaySoundAtLocation` "/Game/Audio/LIghtOn.LIghtOn" (`self.K2_GetActorLocation` _array_element) (struct) 1.0 1.0 0.0 null null null null)
    (`/Game/Audio/BP_LightSoundManager.Light On` (`self.Light Sound Manager`))))

(fn `UserConstructionScript`)