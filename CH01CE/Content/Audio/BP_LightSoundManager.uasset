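; Audio manager that controls a 2D white-noise sound tied to the level's spotlights.
; On BeginPlay it gathers all SpotLight actors and spawns the sound once if any has intensity above zero.
; LightOn spawns the sound if invalid or replays it if stopped, printing a debug message if already playing.
; LightOff fades the playing sound out over a short time.
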(event `self.ReceiveBeginPlay`
  (bind _outactors (`GameplayStatics.GetAllActorsOfClass` "/Script/Engine.SpotLight"))
  (bind _output_get (set `self.Lights` _outactors))
  (for _array_element _output_get
    (if (> (`LightComponentBase.Intensity` (`Light.LightComponent` _array_element)) 0.0)
      (bind _returnvalue (`GameplayStatics.SpawnSound2D` "/Game/Audio/LightWhiteNoise.LightWhiteNoise" 1.0 1.0 0.0 null :!label _label))
      (set `self.LightWhiteNoise` _returnvalue)
      (break))))

(event `Light On`
  (bind _lightwhitenoise (`self.LightWhiteNoise`))
  (if (`KismetSystemLibrary.IsValid` _lightwhitenoise)
    (if (`AudioComponent.IsPlaying` _lightwhitenoise)
      (`KismetSystemLibrary.PrintString` "Hello")
      (else
        (`AudioComponent.Play` _lightwhitenoise 0.0)))
    (else
      (goto _label))))

(event `Light Off`
  (bind _lightwhitenoise (`self.LightWhiteNoise`))
  (if (`KismetSystemLibrary.IsValid` _lightwhitenoise)
    (if (`AudioComponent.IsPlaying` _lightwhitenoise)
      (`AudioComponent.FadeOut` _lightwhitenoise 0.5 0.0 "Linear"))))

(fn `UserConstructionScript`)